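; Default player character Blueprint that handles movement, mouse or stick look, and a sprint input.
; Forward and strafe axes add movement input along the control rotation's forward and right vectors, scaled by PlayerSpeedMultiplier.
; Sprint works as a hold, raising that multiplier on press and resetting it on release, so it scales input rather than changing movement component speed.
; Look axes feed controller pitch and yaw directly.
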(event `InputAxis|MoveForward`
  (params (AxisValue :type "Float (single-precision)"))
  (`self.AddMovementInput` (`KismetMathLibrary.GetForwardVector` (`self.GetControlRotation`)) (* AxisValue (`self.playerSpeedMultiplier`))))

(event `InputAxis|StrafeRight`
  (params (AxisValue :type "Float (single-precision)"))
  (`self.AddMovementInput` (`KismetMathLibrary.GetRightVector` (`self.GetControlRotation`)) (* AxisValue (`self.playerSpeedMultiplier`))))

(event `InputAction|sprintToggle`
  (params (Key :type "Key Structure"))
  (:`Pressed`
    (set `self.playerSpeedMultiplier` 50.0))
  (:`Released`
    (set `self.playerSpeedMultiplier` 1.0)))

(event `InputAxis|lookUp`
  (params (AxisValue :type "Float (single-precision)"))
  (`self.AddControllerPitchInput` AxisValue))

(event `InputAxis|lookLeft`
  (params (AxisValue :type "Float (single-precision)"))
  (`self.AddControllerYawInput` AxisValue))

(fn `UserConstructionScript`)